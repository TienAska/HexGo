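; BP_PlayerController places chess pieces on a grid at the position under the mouse cursor.
; Each tick it traces from the cursor, snaps the hit to the grid and writes the snapped position to the MPC_Cursor material parameter collection.
; Left click spawns a BP_Chess at the snapped XY and traced height, with a running count alternating its IsRed flag.
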(event EventBeginPlay)

(event EventTick
  (params (DeltaSeconds :type Float%20%28single-precision%29))
  (bind (_worldlocation _worlddirection) (Game|Player|ConvertMouseLocationToWorldSpace))
  (bind _outhit (Collision|LineTraceByChannel _worldlocation (+ _worldlocation (* _worlddirection 1e+05)) "TraceTypeQuery1" false 0 "None"))
  (bind _returnvalue (Class|HexBlueprintLibrary|SnapetoGrid (.location _outhit) 1.1e+02))
  (Rendering|Material|SetVectorParameterValue "/Game/Hex/Materials/MPC_Cursor.MPC_Cursor" "WorldPos" (Math|Conversions|ToLinearColor(Vector) (Math|Vector|MakeVector (.x _returnvalue) (.y _returnvalue) (.z _returnvalue))) :!class /Script/Engine.KismetMaterialLibrary)
  (Variables|Default|SetWorldPos (Math|Vector|MakeVector (.x _returnvalue) (.y _returnvalue) (.Z (Math|Vector|BreakVector (.location _outhit))))))

(event Input|MouseEvents|LeftMouseButton
  (params (Key :type Key%20Structure :default "None"))
  (:Pressed
    (bind _returnvalue (Game|SpawnActorfromClass "/Game/Hex/Blueprints/BP_Chess.BP_Chess_C" (Math|Transform|MakeTransform (Variables|Default|GetWorldPos) "0, 0, 0" "1,1,1") "Undefined" 0 0))
    (bind _result (Math|Integer|IncrementInt (Variables|Default|GetChessCount))
      (:%20%20
        (Variables|/Game/Hex/Blueprints/BP_Chess.BP_Chess_C|SetIsRed _returnvalue (> (Math|Integer|%(Integer) _result 2) 0))))))

(fn ConstructionScript)